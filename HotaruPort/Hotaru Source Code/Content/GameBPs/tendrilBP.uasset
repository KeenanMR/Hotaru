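; Growling tendril enemy that leans toward and stretches after the player, knocking them back and damaging them on contact.
; A detection sphere's active state switches Tick between look-at rotation and setting a looping timer that extrudes Z scale, with stretch reset on exit.
; Any damage kills it, hiding mesh and disabling collision until Respawn restores them.
; Retraction and tip-overlap attack logic are unfinished or disconnected.
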(event OnComponentBeginOverlap(attack_hitbox)
  (params (OverlappedComponent :type Primitive%20Component%20Object%20Reference) (OtherActor :type Actor%20Object%20Reference) (OtherComp :type Primitive%20Component%20Object%20Reference) (OtherBodyIndex :type Integer) (bFromSweep :type Boolean) (SweepResult :type Hit%20Result%20Structure%20%28by%20ref%29))
  ;[1 1 1] collision logic for tendril tip
)

(event OnComponentBeginOverlap(player_detection_radius)
  (params (OverlappedComponent :type Primitive%20Component%20Object%20Reference) (OtherActor :type Actor%20Object%20Reference) (OtherComp :type Primitive%20Component%20Object%20Reference) (OtherBodyIndex :type Integer) (bFromSweep :type Boolean) (SweepResult :type Hit%20Result%20Structure%20%28by%20ref%29))
  ;[1 1 1] activates the tendril to go towards the player when within detection radius
  (Components|Activation|Activate (Variables|Default|Getplayer_detection_radius) false)
  (bind _asplayer_character (Utilities|Casting|CastToPlayer_Character OtherActor))
  (Variables|/Game/Player/Player_Model/Player_Character.Player_Character_C|SetCan%20Hit%20Tendril _asplayer_character false)
  (Development|PrintString "hitbox active"))

(event OnComponentEndOverlap(player_detection_radius)
  (params (OverlappedComponent :type Primitive%20Component%20Object%20Reference) (OtherActor :type Actor%20Object%20Reference) (OtherComp :type Primitive%20Component%20Object%20Reference) (OtherBodyIndex :type Integer))
  ;[1 1 1] activates the tendril to go towards the player when within detection radius
  (Components|Activation|Deactivate (Variables|Default|Getplayer_detection_radius))
  (bind _asplayer_character (Utilities|Casting|CastToPlayer_Character OtherActor))
  (Variables|/Game/Player/Player_Model/Player_Character.Player_Character_C|SetCan%20Hit%20Tendril _asplayer_character false)
  (Variables|Default|Setm_stretch 1.0)
  (Development|PrintString "hitbox deactive"))

(event Custom|Respawn
  ;[1 1 1] Respawn Func
  (CallFunction|RespawnTen))

(event Custom|retractTendril
  ;[1 1 1] retracts tendril, doesnt work yet
  (if (not (<= (Variables|Default|Getm_stretch) 1.0))
    (bind _output_get (Variables|Default|Setm_stretch (+ (Variables|Default|Getm_stretch) (* (Variables|Default|Getm_deltaStretch) 2.0))))
    (Development|PrintString (Utilities|String|ToString(Float) _output_get))
    (Transformation|SetActorRelativeScale3D (Math|Vector|MakeVector 1.0 1.0 _output_get))))

(event Custom|extrudeTendril
  ;[1 1 1] stretches up after the player
  (bind _output_get (Variables|Default|Setm_stretch (+ (Variables|Default|Getm_stretch) (Variables|Default|Getm_deltaStretch))))
  (Development|PrintString (Utilities|String|ToString(Float) (Math|Float|Clamp(Float) _output_get 1.0 2.0)) false)
  (Transformation|SetActorRelativeScale3D (Math|Vector|MakeVector 1.0 1.0 (Math|Float|Clamp(Float) _output_get 1.0 2.0))))

(event EventBeginPlay
  (Class|AkGameplayStatics|PostEvent "/Game/Assets/Audio/Events/Play_Lion_Growling_SoundBible_com_657113062.Play_Lion_Growling_SoundBible_com_657113062" self)
  (bind _outactors (Actor|GetAllActorsOfClass "/Game/Player/Player_Model/Player_Character.Player_Character_C"))
  (for _array_element _outactors
    (Variables|Default|SetPlayer _array_element)))

(event Game|Damage|EventAnyDamage
  (params (Damage :type Float%20%28single-precision%29) (DamageType :type Damage%20Type%20Object%20Reference) (InstigatedBy :type Controller%20Object%20Reference) (DamageCauser :type Actor%20Object%20Reference))
  ;[1 1 1] apply damage
  (Variables|Default|Setm_health 0.0)
  (Variables|Default|Setm_isDead true))

(event Collision|EventHit
  (params (MyComp :type Primitive%20Component%20Object%20Reference) (Other :type Actor%20Object%20Reference) (OtherComp :type Primitive%20Component%20Object%20Reference) (bSelfMoved :type Boolean) (HitLocation :type Vector :default "0, 0, 0") (HitNormal :type Vector :default "0, 0, 0") (NormalImpulse :type Vector :default "0, 0, 0") (Hit :type Hit%20Result%20Structure%20%28by%20ref%29))
  ;[1 1 1] detect hit event, pass on information to get hit
  (Class|MTendrilBP|MGetHit Other HitNormal)
  (if (not (Variables|/Script/FirstPlayable.m_Player_Character|Getm_isImmune (Variables|Default|GetPlayer)))
    (Default|Damage (Variables|Default|GetPlayer))))

(event EventTick
  (params (DeltaSeconds :type Float%20%28single-precision%29))
  (if (<= (Variables|Default|Getm_health) 0.0)
    (Class|AkGameplayStatics|PostEvent "/Game/Assets/Audio/Events/Stop_Lion_Growling_SoundBible_com_657113062.Stop_Lion_Growling_SoundBible_com_657113062" self)
    (CallFunction|Death))
  (if (Components|Activation|IsActive (Variables|Default|Getplayer_detection_radius))
    ;[1 1 1] gets the vector from the tendril to the player and makes the tendril lean and face towards the player
    (Transformation|SetWorldRotation (Variables|Transformation|GetRootComponent) (Math|Rotator|FindLookatRotation (Transformation|GetActorLocation) (Transformation|GetActorLocation (Variables|Default|GetPlayer))) false false)
    (else
      ;[1 1 1] stretches up after the player
      (Utilities|Time|SetTimerbyEvent (delegate Custom|extrudeTendril) 0.2 true))))

(fn ConstructionScript)

(fn GetHit
  (params (in_hit :type Actor%20Object%20Reference) (in_hit_normal :type Vector))
  (bind _returnvalue (* in_hit_normal -1e+03))
  (bind (_x _y _z) (Math|Vector|BreakVector _returnvalue))
  ;[1 1 1] knockback player
  (bind _asplayer_character (Utilities|Casting|CastToPlayer_Character in_hit))
  (Variables|Default|Setm_isHitting true)
  (if (Variables|Default|Getm_isHitting)
    (Character|LaunchCharacter _asplayer_character (Math|Vector|MakeVector _x _y (+ _z 5e+01)) true true)))

(fn Death
  (Rendering|SetVisibility (Variables|Default|Gettendril_mesh) false false)
  (Variables|Default|Setm_health 1.0)
  (Collision|SetCollisionEnabled (Variables|Default|Getattack_hitbox) "NoCollision")
  (Collision|SetCollisionEnabled (Variables|Default|Gettendril_mesh) "NoCollision"))

(fn RespawnTen
  (Rendering|SetVisibility (Variables|Default|Gettendril_mesh) true false)
  (Collision|SetCollisionEnabled (Variables|Default|Getattack_hitbox) "QueryAndPhysics")
  (Collision|SetCollisionEnabled (Variables|Default|Gettendril_mesh) "QueryAndPhysics"))